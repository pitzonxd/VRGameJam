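; AC_AILaser is a component that cycles a laser on and off at a spawn point, starting at BeginPlay when that point and the laser class are valid.
; A self-calling FlipFlop alternates between spawning the Laser actor attached to SpawnLocation and destroying that location's first child component, with OnDuration and OffDuration delays.
; The off phase destroys only the component, not the actor, and the cycle stops if no child is found.
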(event Custom|ToggleLaser
  (bind _spawnlocation (Variables|Default|GetSpawnLocation))
  (bind _spawnlocation_2 (Variables|Default|GetSpawnLocation))
  (bind _returnvalue (Components|GetChildComponent _spawnlocation 0))
  (Utilities|FlowControl|FlipFlop
    (:A
      (bind _returnvalue_2 (Game|SpawnActorfromClass (Variables|Components|GetLaser) (Math|Transform|MakeTransform (Transformation|GetWorldLocation _spawnlocation_2) (Transformation|GetWorldRotation _spawnlocation_2) "1.000000,1.000000,1.000000") "Undefined" 0 0))
      (Transformation|AttachComponentToComponent (Variables|/Script/Engine.Actor|GetRootComponent _returnvalue_2) _spawnlocation_2 "None" "SnapToTarget" "SnapToTarget" "KeepWorld" true)
      (Utilities|FlowControl|Delay (Variables|LaserSpawn|GetOn%20Duration))
      (CallFunction|ToggleLaser))
    (:B
      (Utilities|IsValid _returnvalue
        (:Is%20Valid
          (Components|DestroyComponent _returnvalue)
          (Utilities|FlowControl|Delay (Variables|LaserSpawn|GetOff%20Duration))
          (CallFunction|ToggleLaser))))))

(event EventBeginPlay
  (if (and (Utilities|IsValid (Variables|Default|GetSpawnLocation)) (Utilities|IsValidClass (Variables|Components|GetLaser)))
    (CallFunction|ToggleLaser)))