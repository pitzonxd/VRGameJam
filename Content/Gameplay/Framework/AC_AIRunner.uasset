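; Actor component that makes an enemy (Char_EnemyMaster) run back and forth, reversing whenever it is blocked.
; On BeginPlay it caches the owning enemy, then each Tick moves it along its forward vector by Speed and delta time.
; The move is swept, so a blocking hit rotates the enemy 180 degrees.
; A Run function repeats this step without speed or delta scaling and is not called in this graph.
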(event EventBeginPlay
  (bind _aschar_enemy_master (Utilities|Casting|CastToChar_EnemyMaster (Components|GetOwner)))
  (Variables|Default|SetAs%20Char%20Enemy%20Master _aschar_enemy_master))

(event EventTick
  (params (DeltaSeconds :type Float%20%28single-precision%29))
  (bind _as_char_enemy_master (Variables|Default|GetAs%20Char%20Enemy%20Master))
  (bind _sweephitresult (Transformation|AddActorWorldOffset _as_char_enemy_master (* (Transformation|GetActorForwardVector _as_char_enemy_master) DeltaSeconds (Variables|Default|GetSpeed)) true))
  (if (.bBlockingHit (Collision|BreakHitResult _sweephitresult))
    (Class|Actor|AddActorWorldRotation (Variables|Default|GetAs%20Char%20Enemy%20Master) "0,180.000000, 0")))

(fn Run
  (bind _as_char_enemy_master (Variables|Default|GetAs%20Char%20Enemy%20Master))
  (bind _sweephitresult (Transformation|AddActorWorldOffset _as_char_enemy_master (Transformation|GetActorForwardVector _as_char_enemy_master) true))
  (if (.bBlockingHit (Collision|BreakHitResult _sweephitresult))
    (Class|Actor|AddActorWorldRotation _as_char_enemy_master "0,180.000000, 0"))
  (return))