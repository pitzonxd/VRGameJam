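; AC_AIShooter is an actor component that makes its owner fire projectiles at a fixed interval.
; On BeginPlay, given a valid spawn component and projectile class, it enables tick at a custom rate and starts a looping Shoot timer with a randomizable initial delay.
; Tick pauses that timer while the player is beyond a deactivation distance.
; Shoot spawns the projectile at the spawn component's location and rotation, then fires OnShoot.
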(event EventBeginPlay
  (if (and (Utilities|IsValid (Variables|Default|GetSpawnLocation)) (Utilities|IsValidClass (Variables|Components|GetProjectile)))
    (Class|ActorComponent|SetComponentTickInterval (Variables|Performance|GetTickSpeed))
    (Components|Tick|SetComponentTickEnabled true)
    (Utilities|Time|SetTimerbyFunctionName 0 "Shoot" (Variables|ProjectileSpawn|GetShootInterval) true (Variables|ProjectileSpawn|GetInitial%20Start%20Delay) (Variables|ProjectileSpawn|GetInitial%20Start%20Delay%20Variance))))

(event EventTick
  (params (DeltaSeconds :type Float%20%28single-precision%29))
  (bind _returnvalue (Game|GetPlayerCharacter 0))
  (Utilities|IsValid _returnvalue
    (:Is%20Valid
      (if (> (Transformation|GetDistanceTo _returnvalue (Components|GetOwner)) (Variables|Performance|GetDeactivationThreshold))
        (Class|KismetSystemLibrary|PauseTimer 0 "Shoot")
        (else
          (Class|KismetSystemLibrary|UnPauseTimer 0 "Shoot"))))))

(fn Shoot
  (bind _spawnlocation (Variables|Default|GetSpawnLocation))
  (Game|SpawnActorfromClass (Variables|Components|GetProjectile) (Math|Transform|MakeTransform (Transformation|GetWorldLocation _spawnlocation) (Transformation|GetWorldRotation _spawnlocation) (Variables|ProjectileSpawn|GetSpawn%20Transform%20Scale)) "Undefined" 0 0)
  (Default|CallOnShoot)
  (return))